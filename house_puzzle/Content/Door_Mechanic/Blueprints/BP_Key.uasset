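; BP_Key is a key pickup actor for the door mechanic.
; On BeginPlay it creates a P_PickUP prompt widget, which its Box trigger adds to the viewport when the player character enters and removes when they leave.
; Interact calls PickUpKeyMessage on its referenced Door, then destroys the key, with no explicit removal of the prompt.
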(event `/Game/Door_Mechanic/BPI_Interacrt.Interact`
  (message `/Game/Door_Mechanic/BPI_Door.Pick up key` (`self.Door`))
  (`self.K2_DestroyActor`))

(event `self.ReceiveBeginPlay`
  (bind _returnvalue (`|CreateWidget` "/Game/Door_Mechanic/P_PickUP.P_PickUP_C"))
  (set `self.Pick Up` _returnvalue))

(event `self.Box.OnComponentBeginOverlap`
  (params (OverlappedComponent :type "PrimitiveComponent Object Reference") (OtherActor :type "Actor Object Reference") (OtherComp :type "PrimitiveComponent Object Reference") (OtherBodyIndex :type Integer) (bFromSweep :type Boolean) (SweepResult :type "HitResult Structure (by ref)"))
  (if (== OtherActor (`GameplayStatics.GetPlayerCharacter` 0))
    (`UserWidget.AddToViewport` (`self.Pick Up`) 0)))

(event `self.Box.OnComponentEndOverlap`
  (params (OverlappedComponent :type "PrimitiveComponent Object Reference") (OtherActor :type "Actor Object Reference") (OtherComp :type "PrimitiveComponent Object Reference") (OtherBodyIndex :type Integer))
  (if (== (`GameplayStatics.GetPlayerCharacter` 0) OtherActor)
    (`Widget.RemoveFromParent` (`self.Pick Up`))))

(fn `UserConstructionScript`)